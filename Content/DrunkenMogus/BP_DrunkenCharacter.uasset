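; BP_DrunkenCharacter is a character Blueprint that lets the player toggle a focus point in the world with the F key.
; When not focused, F line-traces on Visibility from the follow camera along its forward vector out to FocusRange, with debug drawing on.
; A blocking hit sets IsFocused and stores FocusLocation, and pressing F again clears the flag.
; This graph only sets the focus state and does not act on it.
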(event EventBeginPlay)

(event Collision|EventActorBeginOverlap
  (params (OtherActor :type Actor%20Object%20Reference)))

(event EventTick
  (params (DeltaSeconds :type Float%20%28single-precision%29)))

(event Input|KeyboardEvents|F
  (params (Key :type Key%20Structure :default "None"))
  (bind _followcamera (Variables|Default|GetFollowCamera))
  (bind _returnvalue (Transformation|GetWorldLocation _followcamera))
  (:Pressed
    (if (Variables|Default|GetIsFocused)
      (Variables|Default|SetIsFocused false)
      (else
        (bind _outhit (Collision|LineTraceByChannel _returnvalue (+ _returnvalue (* (Math|Vector|GetForwardVector _followcamera) (Variables|Default|GetFocusRange))) "TraceTypeQuery1" false 0 "ForDuration"))
        (if (.bBlockingHit (Collision|BreakHitResult _outhit))
          (Variables|Default|SetIsFocused true)
          (Variables|Default|SetFocusLocation (.Location (Collision|BreakHitResult _outhit))))))))

(fn ConstructionScript)